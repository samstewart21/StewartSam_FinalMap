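; Puzzle door Blueprint made of six pieces that slide apart to open and back to close.
; BeginPlay records each piece's relative start location, and the OpenDoor timeline lerps the pieces to their end vectors.
; OpenDoor3 sets the opening rate and plays a sound, Finished switches to the closing rate, and CloseDoor3 reverses the timeline.
; A delayed auto-close with closing sound is left unconnected.
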(event `self.ReceiveBeginPlay`
  ;[1 1 1] Figures out the door pieces current location in level and sets it.
  (set `self.TLeftBegin` (`SceneComponent.RelativeLocation` (`self.TopLeft`)))
  (set `self.TMiddleBegin` (`SceneComponent.RelativeLocation` (`self.TopMiddle`)))
  (set `self.TRightBegin` (`SceneComponent.RelativeLocation` (`self.TopRight`)))
  (set `self.BLeftBegin` (`SceneComponent.RelativeLocation` (`self.BottomLeft`)))
  (set `self.BMiddleBegin` (`SceneComponent.RelativeLocation` (`self.BottomMiddle`)))
  (set `self.BRightBegin` (`SceneComponent.RelativeLocation` (`self.BottomRight`))))

(event `OpenDoor3`
  ;[1 1 1] Sets Door Pieces Beginning and End Location
  ;;[0 1 0.1432] Opens Door
  (`TimelineComponent.SetPlayRate` (`self.OpenDoor`) (`self.DoorOpenPlayRate`))
  (`GameplayStatics.PlaySound2D` "/Game/00_One-Sheets/StewartSam_OneSheet03/Audio/DoorOpening.DoorOpening" 1.0 1.0 0.0 null null)
  (bind (_direction _opendoor) (`Timeline|OpenDoor` :!label _label)
    (:`Update`
      (`SceneComponent.K2_SetRelativeLocation` (`self.TopLeft`) (`KismetMathLibrary.VLerp` (`self.TLeftBegin`) (`self.TLeftEnd`) _opendoor) false false)
      (`SceneComponent.K2_SetRelativeLocation` (`self.TopMiddle`) (`KismetMathLibrary.VLerp` (`self.TMiddleBegin`) (`self.TMiddleEnd`) _opendoor) false false)
      (`SceneComponent.K2_SetRelativeLocation` (`self.TopRight`) (`KismetMathLibrary.VLerp` (`self.TRightBegin`) (`self.TRightEnd`) _opendoor) false false)
      (`SceneComponent.K2_SetRelativeLocation` (`self.BottomLeft`) (`KismetMathLibrary.VLerp` (`self.BLeftBegin`) (`self.BLeftEnd`) _opendoor) false false)
      (`SceneComponent.K2_SetRelativeLocation` (`self.BottomMiddle`) (`KismetMathLibrary.VLerp` (`self.BMiddleBegin`) (`self.BMiddleEnd`) _opendoor) false false)
      (`SceneComponent.K2_SetRelativeLocation` (`self.BottomRight`) (`KismetMathLibrary.VLerp` (`self.BRightBegin`) (`self.BRightEnd`) _opendoor) false false))
    (:`Finished`
      ;;[1 0 0] Sets the play rate for closing the door.
      (`TimelineComponent.SetPlayRate` (`self.OpenDoor`) (`self.DoorClosePlayRate`)))))

(event `CloseDoor3`
  ;[1 0 0] Closes Door
  (goto _label :!via `Reverse`))

(fn `UserConstructionScript`)