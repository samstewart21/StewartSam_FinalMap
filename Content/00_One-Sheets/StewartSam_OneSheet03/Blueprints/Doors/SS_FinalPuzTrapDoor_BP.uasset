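; Trap door actor for the final puzzle that slides open and closed.
; BeginPlay caches the door's relative location as the start point for a timeline-driven lerp to an end position.
; OpenDoor04 plays a 2D opening sound and runs the timeline forward, while CloseDoor04 reverses it.
; The closing sound sits in unconnected nodes, so closing is silent.
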(event `self.ReceiveBeginPlay`
  ;[1 1 1] Figures out the trap door's current location and sets the begin variable to that location.
  (set `self.TDoorBegin` (`SceneComponent.RelativeLocation` (`self.TrapDoor`))))

(event `OpenDoor04`
  ;[1 1 1] Slides Open Trap Door
  (`GameplayStatics.PlaySound2D` "/Game/00_One-Sheets/StewartSam_OneSheet03/Audio/DoorOpening.DoorOpening" 1.0 1.0 0.0 null null)
  (bind (_direction _slidedoor) (`Timeline|SlideOpenDoor` :!label _label)
    (:`Update`
      (`SceneComponent.K2_SetRelativeLocation` (`self.TrapDoor`) (`KismetMathLibrary.VLerp` (`self.TDoorBegin`) (`self.TDoorEnd`) _slidedoor) false false))))

(event `CloseDoor04`
  ;[1 1 1] Closes Door
  (goto _label :!via `Reverse`))

(fn `UserConstructionScript`)