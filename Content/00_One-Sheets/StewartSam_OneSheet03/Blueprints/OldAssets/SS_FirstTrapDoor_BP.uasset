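; Trap door actor that slides open while something overlaps its trigger box and slides back when the overlap ends.
; BeginPlay caches the door's relative location as the closed position; the SlideOpenDoor timeline lerps it toward TDoorEnd, playing on begin overlap and reversing on end overlap.
; Any overlapping actor triggers it, as the "Character" name checks are left unconnected.
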(event `self.ReceiveBeginPlay`
  ;[1 1 1] Figures out the trap door's current location and sets the begin variable to that location.
  (set `self.TDoorBegin` (`SceneComponent.RelativeLocation` (`self.TrapDoor`))))

(event `self.BoxCollision.OnComponentBeginOverlap`
  (params (OverlappedComponent :type "PrimitiveComponent Object Reference") (OtherActor :type "Actor Object Reference") (OtherComp :type "PrimitiveComponent Object Reference") (OtherBodyIndex :type Integer) (bFromSweep :type Boolean) (SweepResult :type "HitResult Structure (by ref)"))
  ;[1 1 1] Slides Open Trap Door
  (bind (_direction _slidedoor) (`Timeline|SlideOpenDoor` :!label _label)
    (:`Update`
      (`SceneComponent.K2_SetRelativeLocation` (`self.TrapDoor`) (`KismetMathLibrary.VLerp` (`self.TDoorBegin`) (`self.TDoorEnd`) _slidedoor) false false))))

(event `self.BoxCollision.OnComponentEndOverlap`
  (params (OverlappedComponent :type "PrimitiveComponent Object Reference") (OtherActor :type "Actor Object Reference") (OtherComp :type "PrimitiveComponent Object Reference") (OtherBodyIndex :type Integer))
  ;[1 1 1] Slides door back to original position when player leaves trigger box.
  (goto _label :!via `Reverse`))

(fn `UserConstructionScript`)