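; End platform Blueprint that opens the end doors while a character stands on it.
; Its collision box treats any actor whose display name contains "Character" as a trigger.
; On begin overlap it calls DoorOpen on every SS_EndDoor_BP in the level; on end overlap it waits through a short delay, then calls CloseDoor on them all.
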(event `self.CollisionBox.OnComponentBeginOverlap`
  (params (OverlappedComponent :type "PrimitiveComponent Object Reference") (OtherActor :type "Actor Object Reference") (OtherComp :type "PrimitiveComponent Object Reference") (OtherBodyIndex :type Integer) (bFromSweep :type Boolean) (SweepResult :type "HitResult Structure (by ref)"))
  ;[0 1 0.08953] Opens the door
  (if (`KismetStringLibrary.Contains` (`KismetSystemLibrary.GetDisplayName` OtherActor) "Character")
    (bind _outactors (`GameplayStatics.GetAllActorsOfClass` "/Game/00_One-Sheets/StewartSam_OneSheet03/Blueprints/Doors/SS_EndDoor_BP.SS_EndDoor_BP_C"))
    (`/Game/00_One-Sheets/StewartSam_OneSheet03/Blueprints/Doors/SS_EndDoor_BP.DoorOpen` _outactors)))

(event `self.CollisionBox.OnComponentEndOverlap`
  (params (OverlappedComponent :type "PrimitiveComponent Object Reference") (OtherActor :type "Actor Object Reference") (OtherComp :type "PrimitiveComponent Object Reference") (OtherBodyIndex :type Integer))
  ;[0.4792 0 0] Closes the door
  (if (`KismetStringLibrary.Contains` (`KismetSystemLibrary.GetDisplayName` OtherActor) "Character")
    (`KismetSystemLibrary.Delay` 2.0)
    (bind _outactors (`GameplayStatics.GetAllActorsOfClass` "/Game/00_One-Sheets/StewartSam_OneSheet03/Blueprints/Doors/SS_EndDoor_BP.SS_EndDoor_BP_C"))
    (`/Game/00_One-Sheets/StewartSam_OneSheet03/Blueprints/Doors/SS_EndDoor_BP.CloseDoor` _outactors)))

(fn `UserConstructionScript`)