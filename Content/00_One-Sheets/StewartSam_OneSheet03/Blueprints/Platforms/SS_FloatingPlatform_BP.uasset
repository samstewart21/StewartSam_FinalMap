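; A floating platform actor that moves to an end position after something overlaps its collision box.
; BeginPlay stores the platform's relative location as the start point.
; On overlap, a two-second delay leads into the MovePlatform timeline, which lerps the platform's relative location toward PlatformEnd without sweeping.
; The overlap is not filtered by actor, and the graph contains no return movement.
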(event `self.ReceiveBeginPlay`
  ;[1 1 1] Figures out the platforms current location and sets it.
  (set `self.PlatformBegin` (`SceneComponent.RelativeLocation` (`self.Platform`))))

(event `self.CollisionBox.OnComponentBeginOverlap`
  (params (OverlappedComponent :type "PrimitiveComponent Object Reference") (OtherActor :type "Actor Object Reference") (OtherComp :type "PrimitiveComponent Object Reference") (OtherBodyIndex :type Integer) (bFromSweep :type Boolean) (SweepResult :type "HitResult Structure (by ref)"))
  (`KismetSystemLibrary.Delay` 2.0)
  (bind (_direction _moveplatform) (`Timeline|MovePlatform`)
    (:`Update`
      (`SceneComponent.K2_SetRelativeLocation` (`self.Platform`) (`KismetMathLibrary.VLerp` (`self.PlatformBegin`) (`self.PlatformEnd`) _moveplatform) false false))))

(fn `UserConstructionScript`)