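; Green puzzle-piece pickup sphere that counts toward opening the final puzzle trapdoor.
; A one-shot overlap by an actor with "Character" in its name increments the player character's TrapDoorPuzNum and calls AddGreenSphere on a pickup HUD widget created at BeginPlay.
; When the count reaches NumPuzzlePieces, it shows a puzzle-solved widget and calls OpenDoor04 on each trapdoor actor.
; The piece destroys itself after pickup.
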(event `self.ReceiveBeginPlay`
  ;[1 1 1] Allows access to the Green Puz Piece Widget in this blueprint.
  (bind _returnvalue (`|CreateWidget` "/Game/AAGAM3362/00_One-Sheets/StewartSam_OneSheet02/UIWidgets/OldAssets/SS_Green_PuzPiece_ItemPickup_HUD.SS_Green_PuzPiece_ItemPickup_HUD_C"))
  (set `self.GreenPuzPieceWidget` _returnvalue))

(event `self.SphereCollison.OnComponentBeginOverlap`
  (params (OverlappedComponent :type "PrimitiveComponent Object Reference") (OtherActor :type "Actor Object Reference") (OtherComp :type "PrimitiveComponent Object Reference") (OtherBodyIndex :type Integer) (bFromSweep :type Boolean) (SweepResult :type "HitResult Structure (by ref)"))
  ;[1 1 1] Adds 1 to the trapdoor variable each time a green sphere is picked up
  (`/Engine/EditorBlueprintResources/StandardMacros.DoOnce` false
    (:`Completed`
      (if (`KismetStringLibrary.Contains` (`KismetSystemLibrary.GetObjectName` OtherActor) "Character")
        (bind _asfirst_person_character_h (cast `/Game/FirstPersonBP/Blueprints/FirstPersonCharacter_h` (`GameplayStatics.GetPlayerCharacter` 0)))
        (bind _result (`/Engine/EditorBlueprintResources/StandardMacros.IncrementInt` (`/Game/FirstPersonBP/Blueprints/FirstPersonCharacter_h.TrapDoorPuzNum` _asfirst_person_character_h))
          (:`  `
            (`/Game/AAGAM3362/00_One-Sheets/StewartSam_OneSheet02/UIWidgets/OldAssets/SS_Green_PuzPiece_ItemPickup_HUD.AddGreenSphere` (`self.GreenPuzPieceWidget`))
            (if (>= _result (`self.NumPuzzlePieces`))
              (bind _outactors (`GameplayStatics.GetAllActorsOfClass` "/Game/AAGAM3362/00_One-Sheets/StewartSam_OneSheet02/Blueprints/Doors/SS_FinalPuzTrapDoor_BP.SS_FinalPuzTrapDoor_BP_C"))
              (for _array_element _outactors
                (bind _returnvalue (`|CreateWidget` "/Game/AAGAM3362/00_One-Sheets/StewartSam_OneSheet02/UIWidgets/SS_PuzzleSolved2.SS_PuzzleSolved2_C"))
                (`UserWidget.AddToViewport` _returnvalue 0)
                (`/Game/AAGAM3362/00_One-Sheets/StewartSam_OneSheet02/Blueprints/Doors/SS_FinalPuzTrapDoor_BP.OpenDoor04` _array_element)
                (`self.K2_DestroyActor` :!label _label))
              (else
                (goto _label)))))))))

(fn `UserConstructionScript`)