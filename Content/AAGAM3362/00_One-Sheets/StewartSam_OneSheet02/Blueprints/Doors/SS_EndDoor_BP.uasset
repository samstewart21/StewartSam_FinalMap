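; End door Blueprint made of six sliding pieces (top and bottom left, middle, right) that open and then close automatically.
; BeginPlay caches each piece's relative location as its closed position.
; DoorOpen plays the OpenDoor timeline, lerping every piece toward its End location.
; When the timeline finishes, CloseDoor reverses it at a separate close play rate.
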(event `self.ReceiveBeginPlay`
  ;[1 1 1] Figures out the door pieces current location in level and sets it.
  (set `self.TLeftBegin` (`SceneComponent.RelativeLocation` (`self.TopLeft`)))
  (set `self.TMiddleBegin` (`SceneComponent.RelativeLocation` (`self.TopMiddle`)))
  (set `self.TRightBegin` (`SceneComponent.RelativeLocation` (`self.TopRight`)))
  (set `self.BLeftBegin` (`SceneComponent.RelativeLocation` (`self.BottomLeft`)))
  (set `self.BMiddleBegin` (`SceneComponent.RelativeLocation` (`self.BottomMiddle`)))
  (set `self.BRightBegin` (`SceneComponent.RelativeLocation` (`self.BottomRight`))))

(event `DoorOpen`
  ;[1 1 1] Sets Door Pieces Beginning and End Location
  ;;[0.05189 1 0] Opens the door
  (`TimelineComponent.SetPlayRate` (`self.OpenDoor`) (`self.DoorOpenPlayRate`))
  (bind (_direction _opendoor) (`Timeline|OpenDoor`)
    (:`Update`
      (`SceneComponent.K2_SetRelativeLocation` (`self.TopLeft`) (`KismetMathLibrary.VLerp` (`self.TLeftBegin`) (`self.TLeftEnd`) _opendoor) false false)
      (`SceneComponent.K2_SetRelativeLocation` (`self.TopMiddle`) (`KismetMathLibrary.VLerp` (`self.TMiddleBegin`) (`self.TMiddleEnd`) _opendoor) false false)
      (`SceneComponent.K2_SetRelativeLocation` (`self.TopRight`) (`KismetMathLibrary.VLerp` (`self.TRightBegin`) (`self.TRightEnd`) _opendoor) false false)
      (`SceneComponent.K2_SetRelativeLocation` (`self.BottomLeft`) (`KismetMathLibrary.VLerp` (`self.BLeftBegin`) (`self.BLeftEnd`) _opendoor) false false)
      (`SceneComponent.K2_SetRelativeLocation` (`self.BottomMiddle`) (`KismetMathLibrary.VLerp` (`self.BMiddleBegin`) (`self.BMiddleEnd`) _opendoor) false false)
      (`SceneComponent.K2_SetRelativeLocation` (`self.BottomRight`) (`KismetMathLibrary.VLerp` (`self.BRightBegin`) (`self.BRightEnd`) _opendoor) false false))
    (:`Finished`
      ;;[1 1 1] Sets the play rate and closes the door
      (`TimelineComponent.SetPlayRate` (`self.OpenDoor`) (`self.DoorClosePlayRate`))
      (`self.CloseDoor`))))

(event `CloseDoor`
  ;[0.3646 0 0] Closes Door
  (`TimelineComponent.Reverse` (`self.OpenDoor`)))

(fn `UserConstructionScript`)