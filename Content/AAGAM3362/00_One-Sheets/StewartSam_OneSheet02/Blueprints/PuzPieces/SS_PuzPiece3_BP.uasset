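; Puzzle piece pickup that counts toward opening the final puzzle trap door.
; On BeginPlay it creates the yellow piece pickup HUD widget.
; The first sphere overlap by a Character increments the player's PuzzlePieceNum, updates that HUD through AddSphere, then destroys the piece.
; When the count reaches NumPuzzlePieces, it also shows a puzzle-solved widget and calls OpenDoor04 for each SS_FinalPuzTrapDoor_BP in the level.
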(event `self.ReceiveBeginPlay`
  ;[1 1 1] Create the Yellow Puz Piece Variable.
  (bind _returnvalue (`|CreateWidget` "/Game/AAGAM3362/00_One-Sheets/StewartSam_OneSheet02/UIWidgets/SS_Yellow_PuzPiece_ItemPickupHUD.SS_Yellow_PuzPiece_ItemPickupHUD_C"))
  (set `self.PuzPiece2Widget` _returnvalue))

(event `self.SphereCollison.OnComponentBeginOverlap`
  (params (OverlappedComponent :type "PrimitiveComponent Object Reference") (OtherActor :type "Actor Object Reference") (OtherComp :type "PrimitiveComponent Object Reference") (OtherBodyIndex :type Integer) (bFromSweep :type Boolean) (SweepResult :type "HitResult Structure (by ref)"))
  ;[1 1 1] Checks to see how many puzzle pieces have been collected.
  (`/Engine/EditorBlueprintResources/StandardMacros.DoOnce` false
    (:`Completed`
      (if (`KismetStringLibrary.Contains` (`KismetSystemLibrary.GetObjectName` OtherActor) "Character")
        (bind _asfirst_person_character (cast `/Game/FirstPersonBP/Blueprints/FirstPersonCharacterdumb` (`GameplayStatics.GetPlayerCharacter` 0)))
        (bind _result (`/Engine/EditorBlueprintResources/StandardMacros.IncrementInt` (`/Game/FirstPersonBP/Blueprints/FirstPersonCharacterdumb.PuzzlePieceNum` _asfirst_person_character))
          (:`  `
            ;[1 1 1] Creates the sphere, adds the puzzle solved widget when puzzle is solved and opens door.
            (`/Game/AAGAM3362/00_One-Sheets/StewartSam_OneSheet02/UIWidgets/SS_Yellow_PuzPiece_ItemPickupHUD.AddSphere` (`self.PuzPiece2Widget`))
            (if (>= _result (`self.NumPuzzlePieces`))
              (bind _outactors (`GameplayStatics.GetAllActorsOfClass` "/Game/AAGAM3362/00_One-Sheets/StewartSam_OneSheet02/Blueprints/Doors/SS_FinalPuzTrapDoor_BP.SS_FinalPuzTrapDoor_BP_C"))
              (for _array_element _outactors
                (bind _returnvalue (`|CreateWidget` "/Game/AAGAM3362/00_One-Sheets/StewartSam_OneSheet02/UIWidgets/SS_PuzzleSolved2.SS_PuzzleSolved2_C"))
                (`UserWidget.AddToViewport` _returnvalue 0)
                (`/Game/AAGAM3362/00_One-Sheets/StewartSam_OneSheet02/Blueprints/Doors/SS_FinalPuzTrapDoor_BP.OpenDoor04` _array_element)
                (`self.K2_DestroyActor` :!label _label))
              (else
                (goto _label)))))))))

(fn `UserConstructionScript`)