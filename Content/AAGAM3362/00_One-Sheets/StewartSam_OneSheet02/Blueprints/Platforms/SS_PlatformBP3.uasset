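; Puzzle pressure platform that opens SS_DoorBP_real3 doors when an actor named like "Character" steps on it.
; Overlap compares PlatformPuzzleNum with the DoorPuzzleNum of each "Third"-tagged door; a match calls DoorOpen on every door of that class.
; A brief correct or incorrect widget reports each comparison.
; Leaving the platform waits briefly, then calls DoorClose on the class if a number matches.
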(event `self.CollisionBox.OnComponentBeginOverlap`
  (params (OverlappedComponent :type "PrimitiveComponent Object Reference") (OtherActor :type "Actor Object Reference") (OtherComp :type "PrimitiveComponent Object Reference") (OtherBodyIndex :type Integer) (bFromSweep :type Boolean) (SweepResult :type "HitResult Structure (by ref)"))
  ;[1 1 1] Opens the door
  (if (`KismetStringLibrary.Contains` (`KismetSystemLibrary.GetDisplayName` OtherActor) "Character")
    ;;[1 0.01578 0] Put tags on all "real" doors and update this code for each door!
    (bind _outactors (`GameplayStatics.GetAllActorsOfClassWithTag` "/Game/AAGAM3362/00_One-Sheets/StewartSam_OneSheet02/Blueprints/Doors/SS_DoorBP_real3.SS_DoorBP_real3_C" "Third"))
    (for _array_element _outactors
      (if (== (`self.PlatformPuzzleNum`) (`/Game/AAGAM3362/00_One-Sheets/StewartSam_OneSheet02/Blueprints/Doors/SS_DoorBP_real3.DoorPuzzleNum` _array_element))
        (bind _outactors_2 (`GameplayStatics.GetAllActorsOfClass` "/Game/AAGAM3362/00_One-Sheets/StewartSam_OneSheet02/Blueprints/Doors/SS_DoorBP_real3.SS_DoorBP_real3_C"))
        (`/Game/AAGAM3362/00_One-Sheets/StewartSam_OneSheet02/Blueprints/Doors/SS_DoorBP_real3.DoorOpen` _outactors_2)
        ;;[0 1 0.2018] Tells the player when the puzzle is solved and the door is open. Removes the widget after a few seconds.
        (bind _returnvalue (`|CreateWidget` "/Game/AAGAM3362/00_One-Sheets/StewartSam_OneSheet02/UIWidgets/SS_Correct.SS_Correct_C"))
        (`UserWidget.AddToViewport` _returnvalue 0)
        (`KismetSystemLibrary.Delay` 1.0)
        (bind _foundwidgets (`WidgetBlueprintLibrary.GetAllWidgetsOfClass` "/Game/AAGAM3362/00_One-Sheets/StewartSam_OneSheet02/UIWidgets/SS_Correct.SS_Correct_C"))
        (`Widget.RemoveFromParent` _foundwidgets)
        (else
          ;;[1 0 0] Tells the player they stepped on the wrong platform.
          (bind _returnvalue_2 (`|CreateWidget` "/Game/AAGAM3362/00_One-Sheets/StewartSam_OneSheet02/UIWidgets/SS_Incorrect.SS_Incorrect_C"))
          (`UserWidget.AddToViewport` _returnvalue_2 0)
          (`KismetSystemLibrary.Delay` 1.0)
          (bind _foundwidgets_2 (`WidgetBlueprintLibrary.GetAllWidgetsOfClass` "/Game/AAGAM3362/00_One-Sheets/StewartSam_OneSheet02/UIWidgets/SS_Incorrect.SS_Incorrect_C"))
          (`Widget.RemoveFromParent` _foundwidgets_2))))))

(event `self.CollisionBox.OnComponentEndOverlap`
  (params (OverlappedComponent :type "PrimitiveComponent Object Reference") (OtherActor :type "Actor Object Reference") (OtherComp :type "PrimitiveComponent Object Reference") (OtherBodyIndex :type Integer))
  ;[1 1 1] Closes the door
  (if (`KismetStringLibrary.Contains` (`KismetSystemLibrary.GetDisplayName` OtherActor) "Character")
    (`KismetSystemLibrary.Delay` 1.0)
    (bind _outactors (`GameplayStatics.GetAllActorsOfClassWithTag` "/Game/AAGAM3362/00_One-Sheets/StewartSam_OneSheet02/Blueprints/Doors/SS_DoorBP_real3.SS_DoorBP_real3_C" "Third"))
    (for _array_element _outactors
      (if (== (`self.PlatformPuzzleNum`) (`/Game/AAGAM3362/00_One-Sheets/StewartSam_OneSheet02/Blueprints/Doors/SS_DoorBP_real3.DoorPuzzleNum` _array_element))
        (bind _outactors_2 (`GameplayStatics.GetAllActorsOfClass` "/Game/AAGAM3362/00_One-Sheets/StewartSam_OneSheet02/Blueprints/Doors/SS_DoorBP_real3.SS_DoorBP_real3_C"))
        (`/Game/AAGAM3362/00_One-Sheets/StewartSam_OneSheet02/Blueprints/Doors/SS_DoorBP_real3.DoorClose` _outactors_2)))))

(fn `UserConstructionScript`)